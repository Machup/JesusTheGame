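; Floor tile for an endless runner that fills itself with random content and keeps the track going.
; Construction picks one blocker, fence or collectible, using three lanes or a fence point, and may add a waterfall-type cascade piece.
; When ThirdPersonCharacter hits EndTrigger, LevelOneGameMode adds a tile and this one destroys itself after a delay.
; GetAttachTransform exposes the attach point; boost spawning is defined but uncalled, and CreateFoliage is empty.
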(event OnComponentBeginOverlap(EndTrigger)
  (params (OverlappedComponent :type Primitive%20Component%20Object%20Reference) (OtherActor :type Actor%20Object%20Reference) (OtherComp :type Primitive%20Component%20Object%20Reference) (OtherBodyIndex :type Integer) (bFromSweep :type Boolean) (SweepResult :type Hit%20Result%20Structure%20%28by%20ref%29))
  (Utilities|Casting|CastToThirdPersonCharacter OtherActor)
  (bind _aslevel_one_game_mode (Utilities|Casting|CastToLevelOneGameMode (Game|GetGameMode)))
  (Default|AddFloorTile _aslevel_one_game_mode)
  (Utilities|FlowControl|Delay 2.0)
  (Actor|DestroyActor))

(fn ConstructionScript
  (CallFunction|SetSpawnPoints)
  (CallFunction|SetCascadeSpawnPoints)
  (CallFunction|SpawnItems/Obstacle)
  (CallFunction|SpawnCascade))

(fn GetAttachTransform
  (return (Transformation|GetWorldTransform (Variables|Default|GetAttachPoint))))

(fn SetSpawnPoints
  (Variables|Default|SetSpawnPoints (Utilities|Array|MakeArray (Transformation|GetRelativeTransform (Variables|Default|GetLeft)) (Transformation|GetRelativeTransform (Variables|Default|GetMiddle)) (Transformation|GetRelativeTransform (Variables|Default|GetRight)))))

(fn SpawnItems/Obstacle
  (bind _spawnpoints (Variables|Default|GetSpawnPoints))
  (bind _spawnpoints_2 (Variables|Default|GetSpawnPoints))
  (bind _returnvalue (Utilities|Array|LastIndex _spawnpoints))
  (bind _returnvalue_2 (Math|Random|RandomIntegerinRange 0 _returnvalue))
  (bind _output (Utilities|Array|Get(acopy) _spawnpoints_2 _returnvalue_2))
  (switch int (Math|Random|RandomIntegerinRange 0 5)
    (:0
      ;[0 1 0.7891] Blockers
      (AddComponent|AddChildActorComponent false _output))
    (:1
      (AddComponent|AddChildActorComponent false _output))
    (:2
      (AddComponent|AddChildActorComponent false _output))
    (:3
      (AddComponent|AddChildActorComponent false (Transformation|GetRelativeTransform (Variables|Default|GetSpawnPoint_Fences))))
    (:4
      ;[0 0.5312 1] Collectibles
      (AddComponent|AddChildActorComponent false _output))
    (:5
      (AddComponent|AddChildActorComponent false _output))))

(fn CreateFoliage)

(fn SetCascadeSpawnPoints
  (Variables|Default|SetCascadeSpawnPoints (Utilities|Array|MakeArray (Transformation|GetRelativeTransform (Variables|Default|GetSpawnPoint_Cascade)) (Transformation|GetRelativeTransform (Variables|Default|GetSpawnPoint_Cascade1)) (Transformation|GetRelativeTransform (Variables|Default|GetSpawnPoint_Cascade2)) (Transformation|GetRelativeTransform (Variables|Default|GetSpawnPoint_Cascade3)) (Transformation|GetRelativeTransform (Variables|Default|GetSpawnPoint_Cascade4)) (Transformation|GetRelativeTransform (Variables|Default|GetSpawnPoint_Cascade5)))))

(fn SpawnCascade
  (bind _cascadespawnpoints (Variables|Default|GetCascadeSpawnPoints))
  (bind _cascadespawnpoints_2 (Variables|Default|GetCascadeSpawnPoints))
  (bind _returnvalue (Utilities|Array|LastIndex _cascadespawnpoints))
  (bind _returnvalue_2 (Math|Random|RandomIntegerinRange 0 _returnvalue))
  (bind _output (Utilities|Array|Get(acopy) _cascadespawnpoints_2 _returnvalue_2))
  (switch int (Math|Random|RandomIntegerinRange 0 2)
    (:0
      ;[0 1 0.2031] Waterfall
      (AddComponent|AddChildActorComponent false _output))
    (:1
      (AddComponent|AddChildActorComponent false _output))))

(fn SetBoostSpawnPoints
  (Variables|Default|SetSpeedPointsPoints (Utilities|Array|MakeArray (Transformation|GetRelativeTransform (Variables|Default|GetLeft)) (Transformation|GetRelativeTransform (Variables|Default|GetMiddle)) (Transformation|GetRelativeTransform (Variables|Default|GetRight)))))

(fn SpawnBoost
  (bind _speedpointspoints (Variables|Default|GetSpeedPointsPoints))
  (bind _speedpointspoints_2 (Variables|Default|GetSpeedPointsPoints))
  (bind _returnvalue (Utilities|Array|LastIndex _speedpointspoints_2))
  (bind _returnvalue_2 (Math|Random|RandomIntegerinRange 0 _returnvalue))
  (bind _output (Utilities|Array|Get(acopy) _speedpointspoints _returnvalue_2))
  (switch int (Math|Random|RandomIntegerinRange 0 2)
    (:0
      ;[0 1 0.7891] Boosts
      (AddComponent|AddChildActorComponent false _output))
    (:1
      (AddComponent|AddChildActorComponent false _output))
    (:2
      (Development|PrintString "Hello"))))