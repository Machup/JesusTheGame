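; Player controller for the main menu's character customization, with UI-only input and a visible cursor.
; On BeginPlay it caches the game instance and the first two CustomCharacter actors.
; Its events forward clothing, hair, accessory and part changes to both characters at once.
; Saving writes both characters' data, waits briefly, then stores their saved parts in the game instance; the build-widget creation code is disconnected.
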(event Custom|AddJacket
  (params (State :type Boolean))
  (Default|AddJacket (Variables|Default|GetCustomChar) State))

(event Custom|AddPants
  (params (State :type Boolean))
  (Default|AddPants (Variables|Default|GetCustomChar) State))

(event Custom|SaveSelectedChar
  (Default|SaveCharData (Variables|Default|GetCustomChar2))
  (Utilities|FlowControl|Delay 0.2)
  (bind _savedpartsdata (Default|GetSavedParts (Variables|Default|GetCustomChar)))
  (Default|StoreSavedParts (Variables|Default|GetGameInstance) _savedpartsdata))

(event Custom|AddHairStyle2
  (params (State :type Boolean))
  (Default|AddHair (Variables|Default|GetCustomChar) State "/Game/Jesus/Models/MESH_A_03.MESH_A_03"))

(event Custom|AddHairStyle1
  (params (State :type Boolean))
  (Default|AddHair (Variables|Default|GetCustomChar) State "/Game/Jesus/Models/MESH_A_02.MESH_A_02"))

(event Custom|AddSunglasses
  (params (State :type Boolean))
  (Default|AddSunglasses (Variables|Default|GetCustomChar) State))

(event Custom|AddBeard
  (params (State :type Boolean))
  (Default|AddBeard (Variables|Default|GetCustomChar) State))

(event Custom|UpdateCharPart
  (params (UpdateParts :type E_CurrentCharPart%20Enum :default "NewEnumerator0"))
  (Default|UpdateCharPart (Variables|Default|GetCustomChar) UpdateParts))

(event EventBeginPlay
  (bind _aschar_game_instance (Utilities|Casting|CastToCharGameInstance (Game|GetGameInstance)))
  (Variables|Default|SetGameInstance _aschar_game_instance)
  (Utilities|FlowControl|Sequence
    (:then_0
      (Input|SetInputModeUIOnly self 0 "DoNotLock")
      (Variables|Default|SetbShowMouseCursor true))
    (:then_1
      (bind _outactors (Actor|GetAllActorsOfClass "/Game/Jesus/CustomCharacter.CustomCharacter_C"))
      (Variables|Default|SetCustomChar (Utilities|Array|Get(acopy) _outactors))
      (Variables|Default|SetCustomChar2 (Utilities|Array|Get(acopy) _outactors 1)))))

(fn ConstructionScript)